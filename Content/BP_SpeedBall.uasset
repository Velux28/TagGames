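; BP_SpeedBall is an area actor that speeds up BP_Enemy characters while they overlap it.
; On begin overlap it adds SpeedIncreace to the enemy's CharacterMovement MaxWalkSpeed and prints a debug message.
; On end overlap it subtracts the same amount, so the boost lasts only while the enemy stays inside.
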(event `self.ReceiveActorBeginOverlap`
  (params (OtherActor :type "Actor Object Reference"))
  (bind _asbp_enemy (cast `/Game/BP_Enemy` OtherActor))
  (bind _charactermovement (`Character.CharacterMovement` _asbp_enemy))
  (set `CharacterMovementComponent.MaxWalkSpeed` (+ (`CharacterMovementComponent.MaxWalkSpeed` _charactermovement) (`self.SpeedIncreace`)) _charactermovement)
  (`KismetSystemLibrary.PrintString` "Hey Cowboy Speed Up"))

(event `self.ReceiveActorEndOverlap`
  (params (OtherActor :type "Actor Object Reference"))
  (bind _asbp_enemy (cast `/Game/BP_Enemy` OtherActor))
  (bind _charactermovement (`Character.CharacterMovement` _asbp_enemy))
  (set `CharacterMovementComponent.MaxWalkSpeed` (- (`CharacterMovementComponent.MaxWalkSpeed` _charactermovement) (`self.SpeedIncreace`)) _charactermovement))

(fn `UserConstructionScript`)